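; VR claymore sword actor that can be grabbed, rested on an anvil and given runes.
; On grab it snaps to the SwordSocket of the controller's hand component or the controller itself, and on drop it simulates physics.
; Hitting the old anvil while not held attaches it to the anvil mesh.
; AddRune fills four rune slots in order, and TestRunes checks a four-rune combination.
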(event OnGrabbed(GrabComponentSword)
  (bind _grabcomponentsword (Variables|Default|GetGrabComponentSword))
  (bind _motioncontrollerref (Variables|/Game/VRTemplate/Blueprints/GrabComponent.GrabComponent_C|GetMotionControllerRef _grabcomponentsword))
  (bind _children (Components|GetChildrenComponents _motioncontrollerref false))
  (bind (_array_element _array_index) (Utilities|Array|ForEachLoopwithBreak _children :!label _label)
    (:LoopBody
      (if (Utilities|String|Contains (Utilities|GetObjectName _array_element) "hand")
        (goto _label Break)))
    (:Completed
      (bind _returnvalue (Transformation|AttachComponentToComponent (Variables|Default|GetStaticMeshClaymore) (Utilities|Array|Get(acopy) _children (Variables|Default|GetArray%20Index)) "SwordSocket" "SnapToTarget" "SnapToTarget" "SnapToTarget" false))
      (Variables|Default|SetisGrabbed _returnvalue))))

(event OnDropped(GrabComponentSword)
  (Physics|SetSimulatePhysics (Variables|Default|GetStaticMeshClaymore) true)
  (Variables|Default|SetisGrabbed false))

(event OnComponentHit(StaticMeshClaymore)
  (params (HitComponent :type Primitive%20Component%20Object%20Reference) (OtherActor :type Actor%20Object%20Reference) (OtherComp :type Primitive%20Component%20Object%20Reference) (NormalImpulse :type Vector :default "0, 0, 0") (Hit :type Hit%20Result%20Structure%20%28by%20ref%29))
  (if (and (== OtherActor "/Game/Fab/Old_Anvil/old_anvil.old_anvil") (not (Variables|Default|GetisGrabbed)))
    (Transformation|AttachComponentToComponent (Variables|Default|GetStaticMeshClaymore) (Variables|/Game/anvil.anvil_C|Getold_anvil (Variables|Default|GetAnvil)) "Anvil" "KeepRelative" "KeepRelative" "KeepRelative" true)))

(event Collision|EventActorBeginOverlap
  (params (OtherActor :type Actor%20Object%20Reference)))

(event EventTick
  (params (DeltaSeconds :type Float%20%28single-precision%29)))

(event EventBeginPlay
  (bind _returnvalue (Actor|GetActorOfClass "/Game/anvil.anvil_C"))
  (Variables|Default|SetAnvil _returnvalue))

(fn ConstructionScript)

(fn AddRune
  (params (Rune :type ERuneID%20Enum :default "NONE"))
  (switch int (Variables|Default|GetNumberOfRunes)
    (:0
      (Variables|Default|SetRune%201 Rune))
    (:1
      (Variables|Default|SetRune%202 Rune))
    (:2
      (Variables|Default|SetRune%203 Rune))
    (:3
      (Variables|Default|SetRune%204 Rune)))
  (Variables|Default|SetNumberOfRunes (+ (Variables|Default|GetNumberOfRunes) 1)))

(fn TestRunes
  (params (Rune%201 :type ERuneID%20Enum :default "NONE") (Rune%202 :type ERuneID%20Enum :default "NONE") (Rune%203 :type ERuneID%20Enum :default "NONE") (Rune%204 :type ERuneID%20Enum :default "NONE"))
  (return (Math|Boolean|ANDBoolean (Utilities|Enum|Equal(Enum) Rune%201 (Variables|Default|GetRune%201)) (Utilities|Enum|Equal(Enum) (Variables|Default|GetRune%202) Rune%202) (Utilities|Enum|Equal(Enum) (Variables|Default|GetRune%203) Rune%203) (Utilities|Enum|Equal(Enum) (Variables|Default|GetRune%204) Rune%204))))