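; Interactive book actor that flips through an array of page textures forward or backward on the IA_Turn input.
; The construction script creates dynamic materials for the book and three page meshes, then sets the initial textures and positions.
; One timeline, played or reversed, drives each sheet's roll and its material's Angle parameter for the page arc.
; The three sheets are recycled by modulo index, getting retextured, shown and hidden as the view moves.
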(event Input|EnhancedActionEvents|EnhancedInputActionIA_Turn
  (params (ActionValue :type Float%20%28double-precision%29) (ElapsedSeconds :type Float%20%28double-precision%29) (TriggeredSeconds :type Float%20%28double-precision%29) (InputAction :type Input%20Action%20Object%20Reference :default "/Game/VRTemplate/Input/Actions/IA_Turn.IA_Turn"))
  (bind _nextsheet (Utilities|NextSheet))
  (bind _currentview (Variables|Default|GetCurrentView))
  (bind _currentview_2 (Variables|Default|GetCurrentView))
  (bind _timeline_0 (Variables|Default|GetTimeline_0))
  (bind _staticmeshsheets (Variables|Default|GetStaticMeshSheets))
  (bind _returnvalue (Audio|Components|Audio|IsPlaying _timeline_0))
  (bind _output (Utilities|Array|Get(acopy) _staticmeshsheets _nextsheet))
  (bind _returnvalue_2 (not _returnvalue))
  (if (> ActionValue 0.0)
    ;[1 1 1] Input ( Previous Page, Next Page, Leave Interactive Book )
    (if (and (< (Variables|Default|GetCurrentView) (- (Variables|Default|GetSheetNumber) 1)) _returnvalue_2)
      ;;[1 1 1] Start
      (CallFunction|SetSheetSide "Forward" _nextsheet)
      (Development|SetHiddeninGame _output false false)
      (CallFunction|SetSheetTexture (+ 1 _currentview_2))
      (bind (_direction _page_rotate_amount _page_arc _playing) (Timeline|Timeline_0 PlayFromStart)
        (:Update
          ;;[1 1 1] Update
          (if (> _playing 0.5)
            (switch Utilities|FlowControl|Switch|SwitchonETimelineDirection _direction
              (:Forward
                (CallFunction|TurnPage _page_rotate_amount _page_arc (Utilities|CurrentSheet)))
              (:Backward
                (CallFunction|TurnPage _page_rotate_amount _page_arc (Utilities|PreviousSheet))))))
        (:Finished
          ;;[1 1 1] Finish
          (switch Utilities|FlowControl|Switch|SwitchonETimelineDirection _direction
            (:Forward
              (CallFunction|TurnPage _page_rotate_amount _page_arc (Utilities|CurrentSheet))
              (Development|SetHiddeninGame (Utilities|Array|Get(acopy) (Variables|Default|GetStaticMeshSheets) (Utilities|PreviousSheet)) true false)
              (Math|Integer|IncrementInt _currentview))
            (:Backward
              (CallFunction|TurnPage _page_rotate_amount _page_arc (Utilities|PreviousSheet))
              (Development|SetHiddeninGame (Utilities|Array|Get(acopy) (Variables|Default|GetStaticMeshSheets) (Utilities|CurrentSheet)) true false)
              (Math|Integer|DecrementInt _currentview))))))
    (elif (and _returnvalue_2 (> (Variables|Default|GetCurrentView) 1))
      (CallFunction|SetSheetSide "Backward" _nextsheet)
      (Development|SetHiddeninGame _output false false)
      (CallFunction|SetSheetTexture (- _currentview_2 2))
      (Timeline|Timeline_0 ReverseFromEnd))))

(fn ConstructionScript
  (bind _staticmeshsheets (Variables|Default|GetStaticMeshSheets))
  (bind _pagedynamicmaterials (Variables|Default|GetPageDynamicMaterials))
  ;[1 1 1] Creating Dynamic Materials and Initial Setting
  (Variables|Default|SetSheetNumber (/ (Utilities|Array|Length (Variables|Default|GetPagesTextures)) 2))
  (Utilities|Array|Clear (Variables|Default|GetStaticMeshSheets))
  (Utilities|Array|Clear (Variables|Default|GetPageDynamicMaterials))
  (Utilities|Array|Add _staticmeshsheets (Variables|Default|GetStaticMesh_Page))
  (Utilities|Array|Add _staticmeshsheets (Variables|Default|GetStaticMesh_Page1))
  (Utilities|Array|Add _staticmeshsheets (Variables|Default|GetStaticMesh_Page2))
  (bind _returnvalue (Rendering|Material|CreateDynamicMaterialInstance (Variables|Default|GetStaticMesh) 1 "/Game/MagicianLabatory/BP/InteractiveBook/Material/M_BookPage.M_BookPage" "None" :!class /Script/Engine.PrimitiveComponent))
  (Rendering|Material|SetTextureParameterValue _returnvalue "BookContent" (Variables|Default|GetBookContent_1and4Pages))
  (Utilities|FlowControl|Sequence
    (:then_0
      (bind _returnvalue_2 (Rendering|Material|CreateDynamicMaterialInstance (Variables|Default|GetStaticMesh_Page) 0 "/Game/MagicianLabatory/BP/InteractiveBook/Material/MI_BookPage_Anim.MI_BookPage_Anim" "None" :!class /Script/Engine.PrimitiveComponent))
      (Utilities|Array|SetArrayElem _pagedynamicmaterials 0 _returnvalue_2 true)
      (CallFunction|SetSheetTexture)
      (CallFunction|InitSheetPosition)
      (CallFunction|SetSheetSide "Backward"))
    (:then_1
      (bind _returnvalue_3 (Rendering|Material|CreateDynamicMaterialInstance (Variables|Default|GetStaticMesh_Page1) 0 "/Game/MagicianLabatory/BP/InteractiveBook/Material/MI_BookPage_Anim.MI_BookPage_Anim" "None" :!class /Script/Engine.PrimitiveComponent))
      (Utilities|Array|SetArrayElem _pagedynamicmaterials 1 _returnvalue_3 true)
      (CallFunction|SetSheetTexture 1)
      (CallFunction|InitSheetPosition 1))
    (:then_2
      (bind _returnvalue_4 (Rendering|Material|CreateDynamicMaterialInstance (Variables|Default|GetStaticMesh_Page2) 0 "/Game/MagicianLabatory/BP/InteractiveBook/Material/MI_BookPage_Anim.MI_BookPage_Anim" "None" :!class /Script/Engine.PrimitiveComponent))
      (Utilities|Array|SetArrayElem _pagedynamicmaterials 2 _returnvalue_4 true)
      (CallFunction|SetSheetTexture 2)
      (CallFunction|InitSheetPosition 2))))

(fn InitSheetPosition
  (params (Sheet :type Integer))
  (Rendering|Material|SetVectorParameterValue (Utilities|Array|Get(acopy) (Variables|Default|GetPageDynamicMaterials) Sheet) "Position" (Math|Conversions|ToLinearColor(Vector) (+ (Variables|Default|GetPagePosition) (Variables|/Script/Engine.SceneComponent|GetRelativeLocation (Variables|Default|GetDefaultSceneRoot)))) :!class /Script/Engine.MaterialInstanceDynamic))

(fn SetSheetTexture
  (params (Sheet :type Integer))
  (bind _returnvalue (Math|Integer|%(Integer) Sheet 3))
  (bind _returnvalue_2 (* Sheet 2))
  (bind _pagedynamicmaterials (Variables|Default|GetPageDynamicMaterials))
  (bind _output (Utilities|Array|Get(acopy) _pagedynamicmaterials _returnvalue))
  (Rendering|Material|SetTextureParameterValue _output "BackPage" (Utilities|Array|Get(acopy) (Variables|Default|GetPagesTextures) _returnvalue_2))
  (Rendering|Material|SetTextureParameterValue _output "FrontPage" (Utilities|Array|Get(acopy) (Variables|Default|GetPagesTextures) (+ _returnvalue_2 1))))

(fn TurnPage
  (params (PageRotateAmount :type Float%20%28double-precision%29) (PageArc :type Float%20%28single-precision%29) (Sheet :type Integer))
  (bind _staticmeshsheets (Variables|Default|GetStaticMeshSheets))
  (bind _output (Utilities|Array|Get(acopy) _staticmeshsheets Sheet))
  (bind _relativerotation (Variables|/Script/Engine.SceneComponent|GetRelativeRotation _output))
  (Transformation|SetRelativeRotation _output (Math|Rotator|MakeRotator (* PageRotateAmount (* (Math|Float|Absolute(Float) (Variables|Default|GetPage%20Rotate%20Amount)) -1.0)) (.pitch _relativerotation) (.yaw _relativerotation)) false false)
  (Rendering|Material|SetScalarParameterValue (Utilities|Array|Get(acopy) (Variables|Default|GetPageDynamicMaterials) Sheet) "Angle" PageArc :!class /Script/Engine.MaterialInstanceDynamic))

(fn SetSheetSide
  (params (Direction :type ETimelineDirection%20Enum :default "Forward") (Sheet :type Integer))
  (switch Utilities|FlowControl|Switch|SwitchonETimelineDirection Direction
    (:Forward
      (CallFunction|TurnPage 1.0 -0.125 Sheet))
    (:Backward
      (CallFunction|TurnPage -1.0 0.125 Sheet))))